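; BP_DamageTextActor_Stacking is a floating combat text actor that drifts for a limited lifetime, then destroys itself.
; The construction script picks a drift velocity from the damage type, with randomized sideways angles for DoT and reflect and straight upward motion for the others.
; It also passes itself to the BP_DmgTxtTest widget in its DamageText component.
; Tick applies the drift as a local offset and counts down the lifetime.
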(event `self.ReceiveTick`
  (params (DeltaSeconds :type "Float (single-precision)"))
  (`self.K2_AddActorLocalOffset` (* (`self.Directon`) DeltaSeconds))
  (bind _output_get (set `self.RemainingLifetime` (- (stale _output_get) DeltaSeconds)))
  (if (<= _output_get 0.0)
    (`self.K2_DestroyActor`)))

(fn `UserConstructionScript`
  (bind _returnvalue (`KismetMathLibrary.MakeVector` 0.0 0.0 20.0))
  (bind _returnvalue_2 (* (`KismetMathLibrary.Normal` (`KismetMathLibrary.MakeVector` (`KismetMathLibrary.RandomFloatInRange` -0.5 0.5) 0.0 1.0)) 50.0))
  (set `self.Directon` (select `EDmgType` (`self.DmgType`) :`DT_Skill` _returnvalue :`DT_OnHit` _returnvalue :`DT_DoT` _returnvalue_2 :`DT_Heal` (0.0 0.0 30.0) :`DT_Reflect` _returnvalue_2 :`DT_Invulnerable` (0.0 0.0 10.0) :`DT_Evade` (0.0 0.0 10.0)))
  (bind _asbp_dmg_txt_test (cast `/Game/Blueprints/HuD/DmgText/BP_DmgTxtTest` (`WidgetComponent.GetUserWidgetObject` (`self.DamageText`))))
  (set `/Game/Blueprints/HuD/DmgText/BP_DmgTxtTest.DamageTextActor` self _asbp_dmg_txt_test))