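; BP_2DCamera is an orthographic side-view camera actor that follows its owner on the XZ plane, leaning toward the mouse location.
; Each Tick it targets half the owner-to-mouse offset, clamped to Dist, and interpolates there at a fixed Y depth.
; It floors X and Z to whole units, apparently for pixel snapping.
; Viewport size and ZoomFactor drive ortho width, aspect ratio and the clamp distance.
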(event `self.ReceiveBeginPlay`)

(event `self.ReceiveTick`
  (params (DeltaSeconds :type "Float (single-precision)"))
  (bind _cameracomponent (`self.CameraComponent`))
  (bind _zoomfactor (`self.ZoomFactor`))
  (bind _dist (`self.dist`))
  (bind (_sizex _sizey) (`PlayerController.GetViewportSize` (`self.PlayerController`)))
  (bind _returnvalue (`self.K2_GetActorLocation` (`self.GetOwner`)))
  (bind _returnvalue_2 (`KismetMathLibrary.Conv_IntToDouble` _sizex))
  (bind _returnvalue_3 (`KismetMathLibrary.MakeVector` (.x (- (`self.MouseLocation`) _returnvalue)) 0.0 (.z (- (`self.MouseLocation`) _returnvalue))))
  (`/Engine/EditorBlueprintResources/StandardMacros.IsValid` (`self.PlayerController`)
    (:`Is Valid`
      (`self.K2_SetActorLocation` (`KismetMathLibrary.MakeVector` (`KismetMathLibrary.Conv_IntToDouble` (`KismetMathLibrary.FFloor` (.x (`KismetMathLibrary.VInterpTo` (`self.K2_GetActorLocation`) (+ (`KismetMathLibrary.MakeVector` (.x _returnvalue) 0.0 (.z _returnvalue)) (* (select `bool` (> (`KismetMathLibrary.VSize` _returnvalue_3) _dist) :`false` _returnvalue_3 :`true` (* (`KismetMathLibrary.Normal` _returnvalue_3) _dist)) 0.5)) DeltaSeconds 5.0)))) (`self.CameraDistance`) (`KismetMathLibrary.Conv_IntToDouble` (`KismetMathLibrary.FFloor` (.z (`KismetMathLibrary.VInterpTo` (`self.K2_GetActorLocation`) (+ (`KismetMathLibrary.MakeVector` (.x _returnvalue) 0.0 (.z _returnvalue)) (* (select `bool` (> (`KismetMathLibrary.VSize` _returnvalue_3) _dist) :`false` _returnvalue_3 :`true` (* (`KismetMathLibrary.Normal` _returnvalue_3) _dist)) 0.5)) DeltaSeconds 5.0))))))
      (`|ExecutionSequence`
        (:`then_0`
          (`CameraComponent.SetOrthoWidth` _cameracomponent (/ _returnvalue_2 _zoomfactor))
          (`CameraComponent.SetAspectRatio` _cameracomponent (/ _returnvalue_2 (`KismetMathLibrary.Conv_IntToDouble` _sizey)))
          (set `self.dist` (/ _returnvalue_2 (* _zoomfactor (`self.DistScalar`)))))))))

(fn `UserConstructionScript`)