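; BP_2DHuD creates and manages the player's 2D HUD widget, including the inventory toggle.
; Init builds BP_2DHuD_Widget from the character's Attribute and SkillHandler components, only if both exist, then adds it to the viewport with Game and UI input focused on it.
; OpenInventory toggles the widget's inventory, swaps mouse cursor and crosshair visibility to match, and returns whether it is open.
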(fn `Init`
  (params (`Player Controller` :type "/Game/Blueprints/Character/Player/BP_PlayerController Object Reference") (Character :type "/Game/Blueprints/Character/BP_2DCharacter Object Reference"))
  (bind _returnvalue (`self.K2_GetComponentsByClass` Character "/Script/Test2D.AttributeComponent"))
  (bind _returnvalue_2 (`self.K2_GetComponentsByClass` Character "/Script/Test2D.SkillHandlerComponent"))
  (if (> (`KismetArrayLibrary.Array_Length` _returnvalue) 0)
    (if (> (`KismetArrayLibrary.Array_Length` _returnvalue_2) 0)
      (bind _returnvalue_3 (`|CreateWidget` "/Game/Blueprints/HuD/BP_2DHuD_Widget.BP_2DHuD_Widget_C" `Player Controller` (`KismetArrayLibrary.Array_Get` _returnvalue) (`KismetArrayLibrary.Array_Get` _returnvalue_2)))
      (bind _output_get (set `self.HudWidget` _returnvalue_3))
      (`UserWidget.AddToViewport` _output_get 0)
      (`WidgetBlueprintLibrary.SetInputMode_GameAndUIEx` `Player Controller` _output_get))))

(fn `OpenInventory`
  (returns (Open :type Boolean))
  (bind _returnvalue (`UserWidget.GetOwningPlayer` (`self.HudWidget`)))
  (bind _crosshair (`/Game/Blueprints/HuD/BP_2DHuD_Widget.Crosshair` (`self.HudWidget`)))
  (`/Engine/EditorBlueprintResources/StandardMacros.IsValid` (`self.HudWidget`)
    (:`Is Valid`
      (bind _open (`/Game/Blueprints/HuD/BP_2DHuD_Widget.ToggleInventory` (`self.HudWidget`)))
      (if _open
        (set `PlayerController.bShowMouseCursor` true _returnvalue)
        (`Widget.SetVisibility` _crosshair "Hidden")
        (return true)
        (else
          (set `PlayerController.bShowMouseCursor` false _returnvalue)
          (`Widget.SetVisibility` _crosshair "HitTestInvisible")
          (return false))))
    (:`Is Not Valid`
      (return false))))

(fn `UserConstructionScript`)