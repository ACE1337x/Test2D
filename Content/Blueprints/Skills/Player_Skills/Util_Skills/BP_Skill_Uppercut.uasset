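; Uppercut utility skill for the player that propels its owning Character into the air.
; On the start phase of the SkillMovement event, it launches the owner upward at a boosted multiple of its jump velocity, replacing vertical speed while keeping horizontal momentum.
; An unconnected duplicate of the launch logic remains in the graph and never runs.
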(event `self.SkillMovement`
  (params (update :type "ESkillMotion Enum" :default "SM_START") (dt :type "Float (single-precision)") (ToTargetDir :type "Vector Structure") (LastMoveDir :type "Vector Structure"))
  (bind _owner (`self.owner`))
  (`/Engine/EditorBlueprintResources/StandardMacros.IsValid` _owner
    (:`Is Valid`
      (if (`KismetMathLibrary.ClassIsChildOf` (`GameplayStatics.GetObjectClass` _owner) "/Script/Engine.Character")
        (bind _ascharacter (cast `Character` _owner))
        (switch `ESkillMotion` update
          (:`SM_START`
            (`Character.LaunchCharacter` _ascharacter (`KismetMathLibrary.MakeVector` 0.0 0.0 (* (`CharacterMovementComponent.JumpZVelocity` (`Character.CharacterMovement` _ascharacter)) 1.25)) false true)))))))