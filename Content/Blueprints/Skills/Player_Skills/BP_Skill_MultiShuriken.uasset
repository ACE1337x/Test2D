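; Player skill Blueprint for MultiShuriken, a multi-hit shuriken throw; this graph only builds its description text.
; InitSkillDescription concatenates the hit count from GetTotalHits with per-hit damage into SkillDescription.
; Per-hit damage is the character's TotalStats damage multiplied by the skill data's damage coefficient, so the text reflects the stats at the moment it is built.
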(event `self.InitSkillDescription`
  (bind _returnvalue (`self.GetTotalHits`))
  (set `self.skillDescription` (`KismetStringLibrary.Concat_StrStr` "Throw " (`KismetStringLibrary.Conv_IntToString` _returnvalue) " Shuriken that deal " (`KismetStringLibrary.Conv_DoubleToString` (* (`.Damage` (break `PlayerAttributes` (`Test2DCharacter.totalStats` (`self.Test2DCharacter`)))) (`.skillDamageCoefficient` (break `SkillData` (`.skillData` (break `AbstractSkillData` (`self.skillData`))))))) " Damage per hit.")))