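; Player dodge skill that launches the owning character in its last movement direction with a small hop.
; It acts only on the start update of the SkillMovement event, after confirming the owner is a valid Character.
; The launch overrides current velocity, scaling horizontal speed from the movement component's max speed and lift from a fraction of its jump velocity.
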(event `self.SkillMovement`
  (params (update :type "ESkillMotion Enum" :default "SM_START") (dt :type "Float (single-precision)") (ToTargetDir :type "Vector Structure") (LastMoveDir :type "Vector Structure"))
  (bind _owner (`self.owner`))
  (switch `ESkillMotion` update
    (:`SM_START`
      (`/Engine/EditorBlueprintResources/StandardMacros.IsValid` _owner
        (:`Is Valid`
          (if (`KismetMathLibrary.ClassIsChildOf` (`GameplayStatics.GetObjectClass` _owner) "/Script/Engine.Character")
            (bind _ascharacter (cast `Character` _owner))
            (bind _charactermovement (`Character.CharacterMovement` _ascharacter))
            (`Character.LaunchCharacter` _ascharacter (+ (* LastMoveDir (* (`MovementComponent.GetMaxSpeed` _charactermovement) 2.5)) (`KismetMathLibrary.MakeVector` 0.0 0.0 (/ (`CharacterMovementComponent.JumpZVelocity` _charactermovement) 3.0))) true true)))))))