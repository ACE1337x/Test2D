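; Explosive Kunai player skill Blueprint, whose graph here only builds the skill's description text.
; InitSkillDescription appends literal text with the total hit count as the kunai count and damage computed from the character's Damage stat times the skill coefficient.
; The text describes on-hit damage plus a delayed explosion on the target and those around it, with explosion damage a fixed multiple of hit damage and the delay hardcoded.
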(event `self.InitSkillDescription`
  (bind _returnvalue (* (`.Damage` (break `PlayerAttributes` (`Test2DCharacter.totalStats` (`self.Test2DCharacter`)))) (`.skillDamageCoefficient` (break `SkillData` (`.skillData` (break `AbstractSkillData` (`self.skillData`)))))))
  (bind _returnvalue_2 (`self.GetTotalHits`))
  (set `self.skillDescription` (`KismetStringLibrary.Concat_StrStr` "Throw " (`KismetStringLibrary.Conv_IntToString` _returnvalue_2) " Kunai that deal " (`KismetStringLibrary.Conv_DoubleToString` _returnvalue) " Damage on Hit and Explode after " "2 Seconds dealing " (`KismetStringLibrary.Conv_DoubleToString` (* _returnvalue 10.0)) " Damage to the main target and targets surrounding it.")))