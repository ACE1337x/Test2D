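; Explosive kunai projectile that detonates when destroyed, damaging characters around it.
; On the authority, sphere hits and overlaps call ProjectileHit, and blocking hits also stop the spin.
; Destruction runs Explode, which spawns an explosion emitter and damages Test2DCharacters inside ExplosionSphere, sparing the skill's owner.
; Blast damage scales up the skill's coefficient tenfold and adds evadable knockback, without its own authority check.
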(event `self.ReceiveTick`
  (params (DeltaSeconds :type "Float (single-precision)")))

(event `self.Sphere.OnComponentHit`
  (params (HitComponent :type "PrimitiveComponent Object Reference") (OtherActor :type "Actor Object Reference") (OtherComp :type "PrimitiveComponent Object Reference") (NormalImpulse :type "Vector Structure") (Hit :type "HitResult Structure (by ref)"))
  (`/Engine/EditorBlueprintResources/ActorMacros.Switch Has Authority`
    (:`Authority`
      (`self.ProjectileHit` OtherActor (`.ImpactPoint` (`GameplayStatics.BreakHitResult` Hit)))
      (`self.StopSpinning` null))))

(event `self.Sphere.OnComponentBeginOverlap`
  (params (OverlappedComponent :type "PrimitiveComponent Object Reference") (OtherActor :type "Actor Object Reference") (OtherComp :type "PrimitiveComponent Object Reference") (OtherBodyIndex :type Integer) (bFromSweep :type Boolean) (SweepResult :type "HitResult Structure (by ref)"))
  (`/Engine/EditorBlueprintResources/ActorMacros.Switch Has Authority`
    (:`Authority`
      (`self.ProjectileHit` OtherActor (`.Location` (`GameplayStatics.BreakHitResult` SweepResult))))))

(event `self.StopSpinning`
  (params (attachTo :type "Actor Object Reference"))
  (`parent.StopSpinning` attachTo)
  (`self.NoReally,StopSpinning` null))

(event `NoReally,StopSpinning`
  (params (AttachTo :type "Actor Object Reference"))
  (`parent.StopSpinning` AttachTo)
  (`ActorComponent.Deactivate` (`self.ParticleSystem`)))

(event `self.ReceiveDestroyed`
  (`self.Explode`)
  (`parent.ReceiveDestroyed`))

(fn `Explode`
  (bind _skill (`self.skill`))
  (bind _test2dcharacter (`AbstractSkill.Test2DCharacter` (`self.skill`)))
  (bind _test2dcharacter_2 (`AbstractSkill.Test2DCharacter` _skill))
  (`GameplayStatics.SpawnEmitterAtLocation` "/Game/StarterContent/Particles/P_Explosion.P_Explosion" (`self.K2_GetActorLocation`))
  (for _array_element (`PrimitiveComponent.GetOverlappingActors` (`self.ExplosionSphere`) "/Script/Test2D.Test2DCharacter")
    (if (!= _array_element _test2dcharacter)
      (bind _astest_2dcharacter (cast `Test2DCharacter` _array_element))
      (`Test2DCharacter.TakeDamageTest` _astest_2dcharacter _test2dcharacter (`self.skill`) 0 "DT_Skill" (make `AbstractSkillData` (struct :`skillExtents` (0.0 0.0 0.0) :`nearExtents` (0.0 0.0 0.0) :`orientation` (struct) :`localOffset` (0.0 0.0 0.0) :`skillCollisionType` "SC_Box") (make `SkillInteractionInfo`) (struct) (make `SkillData` :`skillDamageCoefficient` (* (`.skillDamageCoefficient` (break `SkillData` (`.skillData` (break `AbstractSkillData` (`AbstractSkill.skillData` _skill))))) 10.0) :`knockBack` (200.0 0.0 300.0))) (`Test2DCharacter.totalStats` _test2dcharacter_2) (`self.K2_GetActorLocation`) (`Test2DCharacter.damageTextActorStyle` _test2dcharacter_2))))
  (return))

(fn `UserConstructionScript`)