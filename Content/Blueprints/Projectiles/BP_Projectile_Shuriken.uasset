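; Shuriken projectile, a child Blueprint that spins its sprite around the pitch axis every tick until stopped.
; Sphere hit and overlap events run only on authority and pass the other actor and location to ProjectileHit.
; Only a blocking hit also calls StopSpinning, which runs the parent logic and a follow-up event to deactivate the two wisps and particle system.
; An unconnected chain for offsetting those effects never runs.
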(event `self.ReceiveTick`
  (params (DeltaSeconds :type "Float (single-precision)"))
  (if (not (`self.stopped`))
    (`SceneComponent.K2_AddLocalRotation` (`self.Sprite`) (`KismetMathLibrary.MakeRotator` 0.0 (* DeltaSeconds -720.0)) false false)))

(event `self.Sphere.OnComponentHit`
  (params (HitComponent :type "PrimitiveComponent Object Reference") (OtherActor :type "Actor Object Reference") (OtherComp :type "PrimitiveComponent Object Reference") (NormalImpulse :type "Vector Structure") (Hit :type "HitResult Structure (by ref)"))
  (`/Engine/EditorBlueprintResources/ActorMacros.Switch Has Authority`
    (:`Authority`
      (`self.ProjectileHit` OtherActor (`.ImpactPoint` (`GameplayStatics.BreakHitResult` Hit)))
      (`self.StopSpinning` null))))

(event `self.Sphere.OnComponentBeginOverlap`
  (params (OverlappedComponent :type "PrimitiveComponent Object Reference") (OtherActor :type "Actor Object Reference") (OtherComp :type "PrimitiveComponent Object Reference") (OtherBodyIndex :type Integer) (bFromSweep :type Boolean) (SweepResult :type "HitResult Structure (by ref)"))
  (`/Engine/EditorBlueprintResources/ActorMacros.Switch Has Authority`
    (:`Authority`
      (`self.ProjectileHit` OtherActor (`.Location` (`GameplayStatics.BreakHitResult` SweepResult))))))

(event `self.StopSpinning`
  (params (attachTo :type "Actor Object Reference"))
  (`parent.StopSpinning` attachTo)
  (`self.NoReally,StopSpinning` null))

(event `NoReally,StopSpinning`
  (params (AttachTo :type "Actor Object Reference"))
  (`parent.StopSpinning` AttachTo)
  (`ActorComponent.Deactivate` (`self.Wisp0`))
  (`ActorComponent.Deactivate` (`self.Wisp1`))
  (`ActorComponent.Deactivate` (`self.ParticleSystem`)))

(fn `UserConstructionScript`)