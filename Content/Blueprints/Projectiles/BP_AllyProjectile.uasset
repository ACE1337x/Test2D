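; BP_AllyProjectile is an ally projectile, drawn with Paper2D flipbooks, that processes hits on the server.
; Sphere hit and overlap events call ProjectileHit under authority, and only blocking hits also call StopSpinning.
; StopSpinning extends the parent event and triggers a follow-up that deactivates particles and hides the sprite with its children.
; The construction script copies the main sprite's flipbook and color to the Back and Front components.
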(event `self.ReceiveTick`
  (params (DeltaSeconds :type "Float (single-precision)")))

(event `self.Sphere.OnComponentHit`
  (params (OtherActor :type "Actor Object Reference") (OtherComp :type "PrimitiveComponent Object Reference") (NormalImpulse :type "Vector Structure") (Hit :type "HitResult Structure (by ref)"))
  (`/Engine/EditorBlueprintResources/ActorMacros.Switch Has Authority`
    (:`Authority`
      (`self.ProjectileHit` OtherActor (`.ImpactPoint` (`GameplayStatics.BreakHitResult` Hit)))
      (`self.StopSpinning` null))))

(event `self.Sphere.OnComponentBeginOverlap`
  (params (OtherActor :type "Actor Object Reference") (OtherComp :type "PrimitiveComponent Object Reference") (OtherBodyIndex :type Integer) (bFromSweep :type Boolean) (SweepResult :type "HitResult Structure (by ref)"))
  (`/Engine/EditorBlueprintResources/ActorMacros.Switch Has Authority`
    (:`Authority`
      (`self.ProjectileHit` OtherActor (`.Location` (`GameplayStatics.BreakHitResult` SweepResult))))))

(event `self.StopSpinning`
  (params (attachTo :type "Actor Object Reference"))
  (`parent.StopSpinning` attachTo)
  (`self.NoReally,StopSpinning` null))

(event `NoReally,StopSpinning`
  (params (AttachTo :type "Actor Object Reference"))
  (`parent.StopSpinning` AttachTo)
  (`ActorComponent.Deactivate` (`self.ParticleSystem`))
  (`SceneComponent.SetVisibility` (`self.Sprite`) false true))

(fn `UserConstructionScript`
  (bind _sprite (`self.Sprite`))
  (bind _front (`self.Front`))
  (bind _back (`self.Back`))
  (bind _returnvalue (`PaperFlipbookComponent.GetFlipbook` _sprite))
  (bind _spritecolor (`PaperFlipbookComponent.SpriteColor` _sprite))
  (`PaperFlipbookComponent.SetFlipbook` _back _returnvalue)
  (`PaperFlipbookComponent.SetFlipbook` _front _returnvalue)
  (`PaperFlipbookComponent.SetSpriteColor` _back _spritecolor)
  (`PaperFlipbookComponent.SetSpriteColor` _front _spritecolor))