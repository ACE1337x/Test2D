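; Grappling hook skill projectile, cabled to its owner, that destroys itself if the skill already has another projectile out or it exceeds max range.
; On the server, a valid overlap hit or any blocking hit attaches the hook to that actor as the pull target.
; Tick repeatedly launches the owner toward the hook, also pulling overlap-hit characters toward the owner, then stops movement and destroys the hook on arrival.
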(event `self.ReceiveBeginPlay`
  (if (> (`KismetArrayLibrary.Array_Length` (`AbstractSkill.projectiles` (`self.skill`))) 1)
    (`self.K2_DestroyActor`)
    (else
      (set `self.InitialUseLocation` (`self.K2_GetActorLocation`))
      (`CableComponent.SetAttachEndTo` (`self.Cable`) (`self.GetOwner`) "None"))))

(event `self.ReceiveTick`
  (params (DeltaSeconds :type "Float (single-precision)"))
  (`/Engine/EditorBlueprintResources/ActorMacros.Switch Has Authority`
    (:`Authority`
      (`/Engine/EditorBlueprintResources/StandardMacros.IsValid` (`self.PullTo`)
        (:`Is Valid`
          (bind _ascharacter (cast `Character` (`self.GetOwner`)))
          (bind _returnvalue (- (`self.K2_GetActorLocation`) (`self.K2_GetActorLocation` _ascharacter)))
          (if (<= (`KismetMathLibrary.Abs` (`KismetMathLibrary.VSize` _returnvalue)) 10.0)
            (`self.StopMovement` _ascharacter
              (:`OutputPin`
                (`self.K2_DestroyActor`)))
            (else
              (`self.Pull` _ascharacter (* (`KismetMathLibrary.Normal` _returnvalue) 600.0)))))
        (:`Is Not Valid`
          (if (>= (`KismetMathLibrary.VSize` (- (`self.InitialUseLocation`) (`self.K2_GetActorLocation`))) (`self.MaxDistanceToTravel`))
            (`self.K2_DestroyActor`)))))))

(event `self.Sphere.OnComponentBeginOverlap`
  (params (OtherActor :type "Actor Object Reference") (OtherComp :type "PrimitiveComponent Object Reference") (OtherBodyIndex :type Integer) (bFromSweep :type Boolean) (SweepResult :type "HitResult Structure (by ref)"))
  (`/Engine/EditorBlueprintResources/ActorMacros.Switch Has Authority`
    (:`Authority`
      (`/Engine/EditorBlueprintResources/StandardMacros.IsValid` (`self.PullTo`)
        (:`Is Not Valid`
          (bind _stopprojectile (`self.ProjectileHit` OtherActor (`.ImpactPoint` (`GameplayStatics.BreakHitResult` SweepResult))))
          (if _stopprojectile
            (set `self.PullToEachother` true)
            (bind _output_get (set `self.PullTo` OtherActor))
            (`self.K2_AttachRootComponentToActor` _output_get "None" "KeepWorldPosition" false)
            (`MovementComponent.StopMovementImmediately` (`self.ProjectileMovement`))))))))

(event `self.Sphere.OnComponentHit`
  (params (OtherActor :type "Actor Object Reference") (OtherComp :type "PrimitiveComponent Object Reference") (NormalImpulse :type "Vector Structure") (Hit :type "HitResult Structure (by ref)"))
  (`/Engine/EditorBlueprintResources/ActorMacros.Switch Has Authority`
    (:`Authority`
      (`/Engine/EditorBlueprintResources/StandardMacros.IsValid` (`self.PullTo`)
        (:`Is Not Valid`
          (bind _output_get (set `self.PullTo` OtherActor))
          (`self.K2_AttachRootComponentToActor` _output_get "None" "KeepWorldPosition"))))))

(fn `UserConstructionScript`)