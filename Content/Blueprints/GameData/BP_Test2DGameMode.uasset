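; BP_Test2DGameMode is a game mode, named as a 2D test, that sets up a low-quality profiling view and registers players.
; On BeginPlay it runs console commands to show FPS and unit stats, set full screen percentage, and drop several scalability groups to their lowest level.
; Its Loggedin event casts the game state to BP_Test2DGameState and passes the name and controller to AddNetworkedPlayer.
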(event `self.ReceiveBeginPlay`
  (`KismetSystemLibrary.ExecuteConsoleCommand` "stat fps")
  (`KismetSystemLibrary.ExecuteConsoleCommand` "stat unit")
  (`KismetSystemLibrary.ExecuteConsoleCommand` "r.ScreenPercentage 100")
  (`KismetSystemLibrary.ExecuteConsoleCommand` "sg.AntiAliasingQuality 0")
  (`KismetSystemLibrary.ExecuteConsoleCommand` "sg.ViewDistanceQuality 0")
  (`KismetSystemLibrary.ExecuteConsoleCommand` "sg.ShadowQuality 0")
  (`KismetSystemLibrary.ExecuteConsoleCommand` "sg.PostProcessQuality 0")
  (`KismetSystemLibrary.ExecuteConsoleCommand` "sg.EffectsQuality 0")
  (`KismetSystemLibrary.ExecuteConsoleCommand` "sg.TextureQuality 0"))

(event `self.LoggedIn`
  (params (name :type String) (controller :type "PlayerController Object Reference"))
  (bind _asbp_test_2dgame_state (cast `/Game/Blueprints/GameData/BP_Test2DGameState` (`GameplayStatics.GetGameState`)))
  (`/Game/Blueprints/GameData/BP_Test2DGameState.AddNetworkedPlayer` _asbp_test_2dgame_state name controller))

(fn `UserConstructionScript`)