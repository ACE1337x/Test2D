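; Status summon of a floating eye that hovers around the character it is applied to and attacks targetable enemies with its own skill.
; It eases toward a replicated anchor attached to that character, which the server moves to random offsets after randomized delays.
; The server searches characters by distance to owner and eye, then aims and fires the SkillHandler's main slot.
; Server and clients both reposition the light and particles.
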(event EventBeginPlay
  (bind _wantstobe (Variables|Default|GetWantsToBe))
  (Class|ActorComponent|SetIsReplicated (Variables|Default|GetSkillHandler) true)
  (Class|ActorComponent|SetIsReplicated _wantstobe true)
  (Transformation|DetachFromComponent _wantstobe "KeepRelative" "KeepRelative" "KeepRelative" true)
  (Transformation|AttachComponentToComponent _wantstobe (VehicleSound|GetRootComponent (Variables|Default|GetappliedTo)) "None" "KeepRelative" "KeepRelative" "KeepRelative" true)
  (Class|SkillHandlerComponent|Init (Variables|Default|GetSkillHandler) (Variables|Default|GetappliedTo))
  (Networking|SwitchHasAuthority
    (:Authority
      (CallFunction|SetWantstobe))))

(event EventTick
  (params (DeltaSeconds :type Float%20%28single-precision%29))
  (|CallParentFunction DeltaSeconds)
  (CallFunction|FloattoOwner DeltaSeconds)
  (Networking|SwitchHasAuthority
    (:Authority
      (Utilities|FlowControl|Sequence
        (:then_0
          (CallFunction|SearchandDestroy))
        (:then_1
          (Utilities|FlowControl|Delay (Math|Random|RandomFloatinRange 0.5 2.0))
          (CallFunction|SetWantstobe))
        (:then_2
          (CallFunction|MoveLights :!label _label))))
    (:Remote
      (goto _label))))

(fn ConstructionScript)

(fn SearchandDestroy
  (bind _skillhandler (Variables|Default|GetSkillHandler))
  (bind _outactors (Actor|GetAllActorsOfClass "/Script/Test2D.Test2DCharacter"))
  (Utilities|Array|RemoveItem _outactors (Variables|Default|GetappliedBy))
  (for _array_element _outactors
    (Utilities|IsValid _array_element
      (:Is%20Valid
        (bind _returnvalue (Class|Test2DCharacter|CanTarget (Variables|Default|GetappliedBy) _array_element))
        (if _returnvalue
          (if (and (< (Math|Vector|VectorLength (- (Transformation|GetActorLocation (Variables|Default|GetappliedTo)) (Transformation|GetActorLocation _array_element))) (LocalVariables|GetClosestEnemyDistance)) (<= (Math|Vector|VectorLength (- (Transformation|GetActorLocation) (Transformation|GetActorLocation _array_element))) (Variables|Default|GetMaxKillDistance)))
            (LocalVariables|SetClosestEnemyDistance (Math|Vector|VectorLength (- (Transformation|GetActorLocation (Variables|Default|GetappliedTo)) (Transformation|GetActorLocation _array_element))))
            (LocalVariables|SetClosestEnemy _array_element))))))
  (Utilities|IsValid (LocalVariables|GetClosestEnemy)
    (:Is%20Valid
      (bind _output_get (Variables|/Script/Test2D.SkillHandlerComponent|SetToTargetDir _skillhandler (Math|Vector|Normalize (- (Transformation|GetActorLocation (LocalVariables|GetClosestEnemy)) (Transformation|GetActorLocation)))))
      (Class|SkillHandlerComponent|TryUseSkillSlot _skillhandler "SS_Main")
      (bind _returnvalue_2 (Class|SkillHandlerComponent|GetCurrSkill (Variables|Default|GetSkillHandler)))
      (Utilities|IsValid _returnvalue_2
        (:Is%20Valid
          (if (Variables|/Script/Test2D.AbstractSkill|GetbSkillUpdating _returnvalue_2)
            (Transformation|SetActorRotation (Math|Rotator|MakeRotfromX _output_get))
            (else
              (Transformation|SetActorRotation (Variables|/Script/Test2D.Test2DCharacter|GetactorRotation (Variables|Default|GetappliedTo)) :!label _label))))
        (:Is%20Not%20Valid
          (goto _label))))))

(fn SetSpawnLocation
  (Transformation|SetActorLocation (+ (Math|Vector|Normalize (Math|Vector|MakeVector (.X (Math|Vector|BreakVector (Math|Random|RandomUnitVector))) 0.0 0.5)) (Transformation|GetActorLocation)) false false))

(fn FloattoOwner
  (params (Dt :type Float%20%28single-precision%29))
  (bind _returnvalue (Transformation|GetActorLocation))
  (bind _wantstobe (Variables|Default|GetWantsToBe))
  (bind _returnvalue_2 (Transformation|GetWorldLocation _wantstobe))
  (Transformation|SetActorLocation (Math|Interpolation|VInterpTo _returnvalue _returnvalue_2 Dt (/ (Math|Vector|VectorLength (- _returnvalue _returnvalue_2)) 1e+01)) false false))

(fn MoveLights
  (Transformation|SetRelativeLocation (Variables|Default|GetPointLight) (* (Transformation|GetActorRightVector) 1e+01) false false)
  (Transformation|SetRelativeLocation (Variables|Default|GetParticleSystem) (* (Transformation|GetActorRightVector) -2.0) false false))

(fn SetWantstobe
  (Transformation|SetRelativeLocation (Variables|Default|GetWantsToBe) (* (Math|Vector|Normalize (Math|Vector|MakeVector (Math|Random|RandomFloatinRange -1.0 1.0) 0.0 (Math|Random|RandomFloatinRange 0.0 1.0))) (Variables|Default|GetDistanceFromOwner)) false false)
  (return))