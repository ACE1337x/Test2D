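; Bleed status effect that deals damage over time to the character it is applied to.
; On each status tick it calls TakeDamageTest with DoT damage whose skill coefficient scales linearly with the stack count.
; Hits cannot be evaded, carry full defense penetration, and use the applier's damage, crit, lifesteal and damage text style.
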(event `self.TickFunc`
  (bind _appliedby (`self.appliedBy`))
  (bind ((`Damage` _damage) (`Critical_Chance` _critical_chance) (`Critical_Damage` _critical_damage) (`LifeSteal` _lifesteal)) (break `PlayerAttributes` (`Test2DCharacter.totalStats` _appliedby)))
  (`Test2DCharacter.TakeDamageTest` (`self.appliedTo`) (`self.appliedBy`) self 0 "DT_DoT" (make `AbstractSkillData` :`skillData` (make `SkillData` :`skillDamageCoefficient` (* (`KismetArrayLibrary.Array_Length` (`self.stacks`)) 0.1) :`isEvadable` false)) (make `PlayerAttributes` :`Damage` _damage :`Defense_Penetration` 1.0 :`Critical_Chance` _critical_chance :`Critical_Damage` _critical_damage :`LifeSteal` _lifesteal) (0.0 0.0 0.0) (`Test2DCharacter.damageTextActorStyle` _appliedby)))

(fn `UserConstructionScript`)