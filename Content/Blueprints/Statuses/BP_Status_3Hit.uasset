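; BP_Status_3Hit is a stacking status effect, apparently a three-hit mark, that deals bonus damage when it reaches max stacks.
; On max stack it hits the afflicted target with on-hit damage equal to a rounded-up fraction of that target's max HP.
; The hit partially penetrates defense and inherits the owner's crit, life steal and damage-text style, then the status destroys itself.
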(event `self.MaxStackFunc`
  (bind _appliedto (`self.appliedTo`))
  (bind _ownerattribcomp (`self.ownerAttribComp`))
  (bind ((`Critical_Chance` _critical_chance) (`Critical_Damage` _critical_damage) (`LifeSteal` _lifesteal)) (break `PlayerAttributes` (`AttributeComponent.totalStats` _ownerattribcomp)))
  (`AttributeComponent.TakeDamage` :`self` _appliedto :`DamageCauser` _ownerattribcomp :`DamageSource` self :`DmgType` "DT_OnHit" :`otherAttributes` (make `PlayerAttributes` :`Damage` (`KismetMathLibrary.FCeil` (* (`.MaxHP` (break `PlayerAttributes` (`AttributeComponent.totalStats` _appliedto))) (`self.MaxHP%Damage`))) :`Defense_Penetration` 0.5 :`Critical_Chance` _critical_chance :`Critical_Damage` _critical_damage :`LifeSteal` _lifesteal) :`dmgTextActor` (`AttributeComponent.damageTextActorStyle` _ownerattribcomp))
  (`self.K2_DestroyActor`))

(fn `UserConstructionScript`)