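; Bloodrazor passive status that adds bonus on-hit damage based on the victim's max HP whenever its owner's skills hit.
; It binds to the owner's skill-hit delegate on init and unbinds when destroyed.
; Each hit deals rounded-up max-HP-scaled OnHit damage, carrying the owner's penetration, crit and lifesteal stats and damage text style under the same skill use ID.
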(event `self.OnInit`
  (add `Test2DCharacter.onSkillHitDelegate` (`self.appliedTo`) (delegate `OnSkillHit`)))

(event `self.ReceiveDestroyed`
  (remove `Test2DCharacter.onSkillHitDelegate` (`self.appliedTo`) (delegate `OnSkillHit`)))

(event `OnSkillHit`
  (params (hitCharacter :type "Test2DCharacter Object Reference") (skillUseID :type Integer))
  (bind _appliedto (`self.appliedTo`))
  (bind ((`Defense_Penetration` _defense_penetration) (`Critical_Chance` _critical_chance) (`Critical_Damage` _critical_damage) (`LifeSteal` _lifesteal)) (break `PlayerAttributes` (`Test2DCharacter.totalStats` (`self.appliedTo`))))
  (`Test2DCharacter.TakeDamageTest` :`self` hitCharacter :`DamageCauser` _appliedto :`DamageSource` self :`SkillUseID` skillUseID :`DmgType` "DT_OnHit" :`otherAttributes` (make `PlayerAttributes` :`Damage` (`KismetMathLibrary.FCeil` (* (`.MaxHP` (break `PlayerAttributes` (`Test2DCharacter.totalStats` hitCharacter))) (`self.MaxHP%Damage`))) :`Defense_Penetration` _defense_penetration :`Critical_Chance` _critical_chance :`Critical_Damage` _critical_damage :`LifeSteal` _lifesteal) :`dmgTextActor` (`Test2DCharacter.damageTextActorStyle` _appliedto)))

(fn `UserConstructionScript`
  (`parent.UserConstructionScript`))