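; Evasive Maneuver passive status that rewards its owner for evading attacks.
; On init it binds to the owner's take-damage delegate and unbinds when destroyed.
; When a damage event reports the Evade type, the owner applies one timed stack of the stacking damage status to itself through its attribute component.
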(event `self.OnInit`
  (add `Test2DCharacter.onTakeDamageDelegate` (`self.appliedTo`) (delegate `OnEvade`)))

(event `self.ReceiveDestroyed`
  (remove `Test2DCharacter.onTakeDamageDelegate` (`self.appliedTo`) (delegate `OnEvade`)))

(event `OnEvade`
  (params (damageTaken :type "Float (double-precision)") (damageBeforeDefense :type "Float (double-precision)") (damageCauser :type "Test2DCharacter Object Reference") (DamageType :type "EDmgType Enum"))
  (bind _appliedto (`self.appliedTo`))
  (if (`|EnumEquality` DamageType "DT_Evade")
    (`AttributeComponent.applyStatus` (`Test2DCharacter.AttributeComponent` _appliedto) (`|MakeArray` (make `StatusApplicationData` "/Game/Blueprints/Statuses/BP_Status_StackingDamage.BP_Status_StackingDamage_C" 1 10.0)) _appliedto)))

(fn `UserConstructionScript`
  (`parent.UserConstructionScript`))