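; Stacking vampiric status effect that drains its target for the character who applied it.
; Each tick deals unevadable damage over time scaled by stack count, using the owner's stats with full defense penetration and boosted lifesteal.
; At max stacks it spreads itself to targetable characters inside its sphere that have few stacks, hits the host with a larger lifestealing burst, then clears its stacks.
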(event `self.TickFunc`
  (bind _ownerattribcomp (`self.ownerAttribComp`))
  (bind ((`Damage` _damage) (`Critical_Chance` _critical_chance) (`Critical_Damage` _critical_damage) (`LifeSteal` _lifesteal)) (break `PlayerAttributes` (`AttributeComponent.totalStats` _ownerattribcomp)))
  (`AttributeComponent.TakeDamage` (`self.appliedTo`) _ownerattribcomp self 0 "DT_DoT" (make `AbstractSkillData` :`skillData` (make `SkillData` :`skillDamageCoefficient` (* (`KismetArrayLibrary.Array_Length` (`self.stacks`)) 0.05) :`isEvadable` false)) (make `PlayerAttributes` :`Damage` _damage :`Defense_Penetration` 1.0 :`Critical_Chance` _critical_chance :`Critical_Damage` _critical_damage :`LifeSteal` (+ _lifesteal 1.0)) (0.0 0.0 0.0) (`AttributeComponent.damageTextActorStyle` _ownerattribcomp)))

(event `self.MaxStackFunc`
  (bind _ownerattribcomp (`self.ownerAttribComp`))
  (bind _ownerattribcomp_2 (`self.ownerAttribComp`))
  (bind ((`Damage` _damage) (`Critical_Chance` _critical_chance) (`Critical_Damage` _critical_damage) (`LifeSteal` _lifesteal)) (break `PlayerAttributes` (`AttributeComponent.totalStats` _ownerattribcomp_2)))
  (for _array_element (`PrimitiveComponent.GetOverlappingActors` (`self.Sphere`) "/Game/Blueprints/Character/BP_2DCharacter.BP_2DCharacter_C")
    (bind _returnvalue (`self.K2_GetComponentsByClass` _array_element "/Script/Test2D.AttributeComponent"))
    (if (> (`KismetArrayLibrary.Array_Length` _returnvalue) 0)
      (bind _item (`KismetArrayLibrary.Array_Get` _returnvalue))
      (bind _returnvalue_2 (`AttributeComponent.canTarget` _ownerattribcomp _item))
      (if _returnvalue_2
        (bind _returnvalue_3 (`AttributeComponent.getTotalStacksFromStatus` _item (`GameplayStatics.GetObjectClass` self)))
        (if (< _returnvalue_3 5)
          (`AttributeComponent.applyStatus` _item (`|MakeArray` (make `StatusApplicationData` "BP_Status_Vamp_C" 5 10.0)) _ownerattribcomp)))))
  (`AttributeComponent.TakeDamage` (`self.appliedTo`) _ownerattribcomp_2 self 0 "DT_DoT" (make `AbstractSkillData` :`skillData` (make `SkillData` :`skillDamageCoefficient` (* (`KismetArrayLibrary.Array_Length` (`self.stacks`)) 0.5) :`skillIncreasedLifesteal` 1.0 :`isEvadable` false)) (make `PlayerAttributes` :`Damage` _damage :`Defense_Penetration` 1.0 :`Critical_Chance` _critical_chance :`Critical_Damage` _critical_damage :`LifeSteal` _lifesteal) (0.0 0.0 0.0) (`AttributeComponent.damageTextActorStyle` _ownerattribcomp_2))
  (`KismetArrayLibrary.Array_Clear` (`self.stacks`)))

(fn `UserConstructionScript`)