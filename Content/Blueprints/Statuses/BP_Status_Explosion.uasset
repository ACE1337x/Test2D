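; Explosion status effect that detonates in its stack-decrement event, then destroys itself.
; Actors in its sphere whose AttributeComponent is of a different alliance from the owner receive stacks of BP_Status_Bleed.
; Only the afflicted target takes the evadable skill hit with knockback, scaled from the owner's damage, penetration, crit and lifesteal stats.
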(event `self.StackDecrFunc`
  (bind _ownerattribcomp (`self.ownerAttribComp`))
  (bind _ownerattribcomp_2 (`self.ownerAttribComp`))
  (bind ((`Damage` _damage) (`Defense_Penetration` _defense_penetration) (`Critical_Chance` _critical_chance) (`Critical_Damage` _critical_damage) (`LifeSteal` _lifesteal)) (break `PlayerAttributes` (`AttributeComponent.totalStats` _ownerattribcomp_2)))
  (for _array_element (`PrimitiveComponent.GetOverlappingActors` (`self.Sphere`) "/Game/Blueprints/Character/BP_2DCharacter.BP_2DCharacter_C")
    (bind _returnvalue (`self.K2_GetComponentsByClass` _array_element "/Script/Test2D.AttributeComponent"))
    (if (> (`KismetArrayLibrary.Array_Length` _returnvalue) 0)
      (bind _item (`KismetArrayLibrary.Array_Get` _returnvalue))
      (if (and (!= _item _ownerattribcomp) (`|EnumInequality` (`AttributeComponent.AllianceType` _item) (`AttributeComponent.AllianceType` _ownerattribcomp)))
        (`AttributeComponent.applyStatus` _item (`|MakeArray` (make `StatusApplicationData` "/Game/Blueprints/Statuses/BP_Status_Bleed.BP_Status_Bleed_C" 5 10.0)) _ownerattribcomp))))
  (`AttributeComponent.TakeDamage` (`self.appliedTo`) _ownerattribcomp_2 self 0 "DT_Skill" (make `AbstractSkillData` :`skillInteractionInfo` (make `SkillInteractionInfo`) :`skillData` (make `SkillData` :`skillDamageCoefficient` 10.0 :`knockBack` (200.0 0.0 300.0))) (make `PlayerAttributes` :`Damage` _damage :`Defense_Penetration` _defense_penetration :`Critical_Chance` _critical_chance :`Critical_Damage` _critical_damage :`LifeSteal` _lifesteal) (0.0 0.0 0.0) (`AttributeComponent.damageTextActorStyle` _ownerattribcomp_2))
  (`self.K2_DestroyActor`))

(fn `UserConstructionScript`)