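; Bloodrazor passive status that adds bonus on-hit damage scaled to the struck target's maximum HP.
; On init it binds to the owner's skill-hit delegate, and unbinds when destroyed.
; Each skill hit deals a rounded-up fraction of the target's max HP as OnHit damage under the same skill use ID.
; That damage carries the owner's defense penetration, critical stats, lifesteal and damage text style.
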(event `self.OnInit`
  (add `AttributeComponent.onSkillHitDelegate` (`self.appliedTo`) (delegate `OnSkillHit`)))

(event `self.ReceiveDestroyed`
  (remove `AttributeComponent.onSkillHitDelegate` (`self.appliedTo`) (delegate `OnSkillHit`)))

(event `OnSkillHit`
  (params (hitAttribComp :type "AttributeComponent Object Reference") (skillUseID :type Integer))
  (bind _appliedto (`self.appliedTo`))
  (bind ((`Defense_Penetration` _defense_penetration) (`Critical_Chance` _critical_chance) (`Critical_Damage` _critical_damage) (`LifeSteal` _lifesteal)) (break `PlayerAttributes` (`AttributeComponent.totalStats` (`self.appliedTo`))))
  (`AttributeComponent.TakeDamage` :`self` hitAttribComp :`DamageCauser` _appliedto :`DamageSource` self :`SkillUseID` skillUseID :`DmgType` "DT_OnHit" :`otherAttributes` (make `PlayerAttributes` :`Damage` (`KismetMathLibrary.FCeil` (* (`.MaxHP` (break `PlayerAttributes` (`AttributeComponent.totalStats` hitAttribComp))) (`self.MaxHP%Damage`))) :`Defense_Penetration` _defense_penetration :`Critical_Chance` _critical_chance :`Critical_Damage` _critical_damage :`LifeSteal` _lifesteal) :`dmgTextActor` (`AttributeComponent.damageTextActorStyle` _appliedto)))

(fn `UserConstructionScript`
  (`parent.UserConstructionScript`))