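; Thornmail status effect that reflects part of the damage its bearer takes back at the attacker.
; On init it binds to the bearer's take-damage delegate.
; Each non-Reflect hit returns a quarter of the pre-defense damage, rounded up, as an unevadable knockback hit using the bearer's penetration and crit stats.
; The returned hit is typed Skill, so the Reflect check does not filter it on another Thornmail bearer.
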(event `self.OnInit`
  (add `Test2DCharacter.onTakeDamageDelegate` (`self.appliedTo`) (delegate `ReflectDamage`)))

(event `ReflectDamage`
  (params (damageTaken :type "Float (double-precision)") (damageBeforeDefense :type "Float (double-precision)") (damageCauser :type "Test2DCharacter Object Reference") (DamageType :type "EDmgType Enum"))
  (bind _appliedto (`self.appliedTo`))
  (bind ((`Damage_Reduction` _damage_reduction) (`Defense_Penetration` _defense_penetration) (`Critical_Chance` _critical_chance) (`Critical_Damage` _critical_damage)) (break `PlayerAttributes` (`Test2DCharacter.totalStats` _appliedto)))
  (if (`|EnumInequality` DamageType "DT_Reflect")
    (`Test2DCharacter.TakeDamageTest` damageCauser null self 0 "DT_Skill" (make `AbstractSkillData` :`skillData` (make `SkillData` :`knockBack` (50.0 0.0 50.0) :`isEvadable` false)) (make `PlayerAttributes` :`Damage` (`KismetMathLibrary.FCeil` (* damageBeforeDefense 0.25)) :`Defense_Penetration` _defense_penetration :`Critical_Chance` _critical_chance :`Critical_Damage` _critical_damage) (0.0 0.0 0.0) (`Test2DCharacter.damageTextActorStyle` _appliedto))))

(fn `UserConstructionScript`)