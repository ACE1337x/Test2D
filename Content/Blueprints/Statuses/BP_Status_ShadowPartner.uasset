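; Shadow Partner status actor that shows a darkened, semi-transparent copy of its owner's Paper2D sprite trailing just behind it.
; On BeginPlay it copies the owner's first flipbook, derives the shadow tint from its color and snaps to its position.
; Each Tick it interpolates toward a point behind the owner on a fixed Y plane, matches rotation and updates its flipbook to follow the owner's.
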(event `self.ReceiveBeginPlay`
  (`self.SetSprite`))

(event `self.ReceiveTick`
  (params (DeltaSeconds :type "Float (single-precision)"))
  (`/Engine/EditorBlueprintResources/ActorMacros.Switch Has Authority`
    (:`Authority`
      _)
    (:`Remote`
      _))
  (`self.UpdateSprite` DeltaSeconds))

(fn `SetSprite`
  (bind _sprite (`self.Sprite`))
  (bind _output_get (set `self.OwnerFlipbook` (`KismetArrayLibrary.Array_Get` (`self.K2_GetComponentsByClass` (`self.GetOwner`) "/Script/Paper2D.PaperFlipbookComponent"))))
  (`PaperFlipbookComponent.SetFlipbook` _sprite (`PaperFlipbookComponent.GetFlipbook` _output_get))
  (bind (_r _g _b) (`KismetMathLibrary.BreakColor` (`PaperFlipbookComponent.SpriteColor` _output_get)))
  (`PaperFlipbookComponent.SetSpriteColor` _sprite (`KismetMathLibrary.MakeColor` (- _r 0.7) (- _g 0.7) (- _b 0.7) 0.7))
  (`self.K2_SetActorLocation` (`KismetMathLibrary.MakeVector` (.x (`SceneComponent.K2_GetComponentLocation` (`self.OwnerFlipbook`))) -1.0 (.z (`SceneComponent.K2_GetComponentLocation` (`self.OwnerFlipbook`)))) false true)
  (return))

(fn `UpdateSprite`
  (params (DeltaTime :type "Float (double-precision)"))
  (bind _returnvalue (`self.GetOwner`))
  (bind _ownerflipbook (`self.OwnerFlipbook`))
  (bind _sprite (`self.Sprite`))
  (bind _returnvalue_2 (`PaperFlipbookComponent.GetFlipbook` _ownerflipbook))
  (`/Engine/EditorBlueprintResources/StandardMacros.IsValid` _ownerflipbook
    (:`Is Valid`
      (`|ExecutionSequence`
        (:`then_0`
          (`self.K2_SetActorLocation` (`KismetMathLibrary.VInterpTo` (`self.K2_GetActorLocation`) (+ (`KismetMathLibrary.MakeVector` (.x (`SceneComponent.K2_GetComponentLocation` (`self.OwnerFlipbook`))) -1.0 (.z (`SceneComponent.K2_GetComponentLocation` (`self.OwnerFlipbook`)))) (* (`KismetMathLibrary.NegateVector` (`self.GetActorForwardVector` _returnvalue)) 10.0)) DeltaTime 20.0))
          (`self.SetActorRotation` (`self.K2_GetActorRotation` _returnvalue)))
        (:`then_1`
          (if (!= _sprite _returnvalue_2)
            (`PaperFlipbookComponent.SetFlipbook` _sprite _returnvalue_2)))))))

(fn `UserConstructionScript`)