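; BP_Status_FloatEye is a status actor: a floating eye that hovers around its owner and attacks targetable pawns.
; A replicated WantsToBe point on the affected actor's root is re-randomized by the server in an upper X-Z arc, and the eye eases toward it.
; The server picks the pawn nearest the owner within the eye's kill range, fires the main skill, and faces it while that skill updates.
; Detached light and particles follow at fixed world offsets.
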(event EventBeginPlay
  (bind _wantstobe (Variables|Default|GetWantsToBe))
  (Class|ActorComponent|SetIsReplicated _wantstobe true)
  (Class|SceneComponent|DetachfromParent _wantstobe true true)
  (Class|SceneComponent|Attachto _wantstobe (VehicleSound|GetRootComponent (Components|GetOwner (Variables|Default|GetappliedTo))) "None" "SnapToTargetIncludingScale" true)
  (Class|SceneComponent|DetachfromParent (Variables|Default|GetPointLight) true true)
  (Class|SceneComponent|DetachfromParent (Variables|Default|GetParticleSystem) true true)
  (Networking|SwitchHasAuthority
    (:Authority
      (CallFunction|SetWantstobe))))

(event EventTick
  (params (DeltaSeconds :type Float%20%28single-precision%29))
  (|CallParentFunction DeltaSeconds)
  (CallFunction|FloattoOwner DeltaSeconds)
  (CallFunction|MoveLights)
  (Networking|SwitchHasAuthority
    (:Authority
      (Utilities|FlowControl|Sequence
        (:then_0
          (CallFunction|SearchandDestroy))
        (:then_1
          (Utilities|FlowControl|Delay (Math|Random|RandomFloatinRange 0.5 2.0))
          (CallFunction|SetWantstobe))))))

(fn ConstructionScript)

(fn SearchandDestroy
  (bind _self self)
  (bind _skillhandler (Variables|Default|GetSkillHandler))
  (bind _outactors (Actor|GetAllActorsOfClass "/Script/Engine.Pawn"))
  (bind _aspawn (Utilities|Casting|CastToPawn (Components|GetOwner)))
  (Utilities|Array|RemoveItem _outactors _aspawn)
  (for _array_element _outactors
    (if (> (Utilities|Array|Length (Actor|GetComponentsByClass _array_element "/Script/Test2D.AttributeComponent")) 0)
      (bind _returnvalue (Class|AttributeComponent|CanTarget (Variables|Default|GetownerAttribComp) (Utilities|Array|Get(acopy) (Actor|GetComponentsByClass _array_element "/Script/Test2D.AttributeComponent"))))
      (if _returnvalue
        (if (and (< (Math|Vector|VectorLength (- (Transformation|GetActorLocation (Components|GetOwner)) (Transformation|GetActorLocation _array_element))) (LocalVariables|GetClosestEnemyDistance)) (<= (Math|Vector|VectorLength (- (Transformation|GetActorLocation) (Transformation|GetActorLocation _array_element))) (Variables|Default|GetMaxKillDistance)))
          (LocalVariables|SetClosestEnemyDistance (Math|Vector|VectorLength (- (Transformation|GetActorLocation (Components|GetOwner)) (Transformation|GetActorLocation _array_element))))
          (LocalVariables|SetClosestEnemy _array_element)))))
  (Utilities|IsValid (LocalVariables|GetClosestEnemy)
    (:Is%20Valid
      (bind _output_get (Variables|/Script/Test2D.SkillHandlerComponent|SetToTargetDir _skillhandler (Math|Vector|Normalize (- (Transformation|GetActorLocation (LocalVariables|GetClosestEnemy)) (Transformation|GetActorLocation)))))
      (Class|SkillHandlerComponent|TryUseSkillSlot _skillhandler "SS_Main")
      (bind _returnvalue_2 (Class|SkillHandlerComponent|GetCurrSkill (Variables|Default|GetSkillHandler)))
      (Utilities|IsValid _returnvalue_2
        (:Is%20Valid
          (if (Variables|/Script/Test2D.AbstractSkill|GetbSkillUpdating _returnvalue_2)
            (Transformation|SetActorRotation (Math|Rotator|MakeRotator (.Roll (Math|Rotator|BreakRotator (Math|Rotator|MakeRotationfromAxes _output_get (Transformation|GetActorRightVector _self) (Transformation|GetActorUpVector _self)))) (.Pitch (Math|Rotator|BreakRotator (Math|Rotator|MakeRotationfromAxes _output_get (Transformation|GetActorRightVector _self) (Transformation|GetActorUpVector _self)))) (.Yaw (Math|Rotator|BreakRotator (Math|Rotator|MakeRotationfromAxes _output_get (Transformation|GetActorRightVector _self) (Transformation|GetActorUpVector _self))))))
            (else
              (Transformation|SetActorRotation (Transformation|GetActorRotation (Components|GetOwner)) :!label _label))))
        (:Is%20Not%20Valid
          (goto _label))))))

(fn SetSpawnLocation
  (Transformation|SetActorLocation (+ (Math|Vector|Normalize (Math|Vector|MakeVector (.X (Math|Vector|BreakVector (Math|Random|RandomUnitVector))) 0.0 0.5)) (Transformation|GetActorLocation)) false false))

(fn FloattoOwner
  (params (Dt :type Float%20%28single-precision%29))
  (bind _returnvalue (Transformation|GetActorLocation))
  (bind _wantstobe (Variables|Default|GetWantsToBe))
  (bind _returnvalue_2 (Transformation|GetWorldLocation _wantstobe))
  (Transformation|SetActorLocation (Math|Interpolation|VInterpTo _returnvalue _returnvalue_2 Dt (/ (Math|Vector|VectorLength (- _returnvalue _returnvalue_2)) 1e+01)) false false))

(fn MoveLights
  (Transformation|SetWorldLocation (Variables|Default|GetPointLight) (+ (Transformation|GetActorLocation) "0,30.000000, 0") false false)
  (Transformation|SetWorldLocation (Variables|Default|GetParticleSystem) (+ (Transformation|GetActorLocation) "0,-10.000000, 0") false false)
  (return))

(fn SetWantstobe
  (Transformation|SetRelativeLocation (Variables|Default|GetWantsToBe) (* (Math|Vector|Normalize (Math|Vector|MakeVector (Math|Random|RandomFloatinRange -1.0 1.0) 0.0 (Math|Random|RandomFloatinRange 0.0 1.0))) (Variables|Default|GetDistanceFromOwner)) false false)
  (return))