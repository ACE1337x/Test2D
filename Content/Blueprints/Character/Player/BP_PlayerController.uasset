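; Player controller for the 2D game that relays movement, jump, PVP toggle and skill input to the possessed BP_Player_Character.
; Init caches that character and initializes the HUD; the inventory key also toggles the character's camera updates.
; Each skill slot uses a TryUseSkill gate macro driven by Tick, so a held button retries its skill every frame.
; Escape quits the game, and destruction removes the controller from the game state's list.
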(event `Key|Escape`
  (params (Key :type "Key Structure" :default "AnyKey"))
  (:`Pressed`
    (`KismetSystemLibrary.QuitGame` null "Quit")))

(event `Key|I`
  (params (Key :type "Key Structure" :default "AnyKey"))
  (bind _base2dcharacter (`self.Base2DCharacter`))
  (:`Pressed`
    (bind _asbp_2dhu_d (cast `/Game/Blueprints/HuD/BP_2DHuD` (`self.GetHUD`)))
    (bind _open (`/Game/Blueprints/HuD/BP_2DHuD.OpenInventory` _asbp_2dhu_d))
    (`/Engine/EditorBlueprintResources/StandardMacros.IsValid` _base2dcharacter
      (:`Is Valid`
        (`/Game/Blueprints/Character/Player/BP_Player_Character.ToggleUpdateCamera` _base2dcharacter (not _open))))))

(event `Key|P`
  (params (Key :type "Key Structure" :default "AnyKey"))
  (:`Pressed`
    (`Test2DCharacter.TogglePVP` (`self.Base2DCharacter`))))

(event `Walk`
  (params (AxisValue :type "Float (double-precision)"))
  (bind _base2dcharacter (`self.Base2DCharacter`))
  (`/Engine/EditorBlueprintResources/StandardMacros.IsValid` _base2dcharacter
    (:`Is Valid`
      (`Test2DCharacter.MoveRight` _base2dcharacter AxisValue))))

(event `InputAxis|MoveRight`
  (params (AxisValue :type "Float (single-precision)"))
  (`self.Walk` AxisValue))

(event `MoveUp`
  (params (`Axis Value` :type "Float (double-precision)"))
  (bind _base2dcharacter (`self.Base2DCharacter`))
  (`/Engine/EditorBlueprintResources/StandardMacros.IsValid` _base2dcharacter
    (:`Is Valid`
      (`Test2DCharacter.MoveUp` _base2dcharacter `Axis Value`))))

(event `InputAxis|MoveUp`
  (params (AxisValue :type "Float (single-precision)"))
  (`self.MoveUp` AxisValue))

(event `self.ReceiveTick`
  (params (DeltaSeconds :type "Float (single-precision)"))
  (`|ExecutionSequence`
    (:`then_0`
      (`self.TryUseSkill` "SS_Main" :!label _label))
    (:`then_1`
      (`self.TryUseSkill` "SS_Secondary" :!label _label_2))
    (:`then_2`
      (`self.TryUseSkill` "SS_Util_0" :!label _label_3))
    (:`then_3`
      (`self.TryUseSkill` "SS_Util_1" :!label _label_4))
    (:`then_4`
      (`self.TryUseSkill` "SS_Util_2" :!label _label_5))
    (:`then_5`
      (`self.TryUseSkill` "SS_Dodge" :!label _label_6))
    (:`then_6`
      (`self.TryUseSkill` "SS_Buff_0" :!label _label_7))
    (:`then_7`
      (`self.TryUseSkill` "SS_Buff_1" :!label _label_8))
    (:`then_8`
      (`self.TryUseSkill` "SS_Buff_2" :!label _label_9))))

(event `Jump`
  (bind _base2dcharacter (`self.Base2DCharacter`))
  (`/Engine/EditorBlueprintResources/StandardMacros.IsValid` _base2dcharacter
    (:`Is Valid`
      (`Test2DCharacter.Jump` _base2dcharacter))))

(event `InputAction|Skill_Main`
  (params (Key :type "Key Structure" :default "AnyKey"))
  (:`Pressed`
    (goto _label :!via `Press`))
  (:`Released`
    (goto _label :!via `Release`)))

(event `InputAction|Jump`
  (params (Key :type "Key Structure" :default "AnyKey"))
  (:`Pressed`
    (`self.Jump`)))

(event `InputAction|Skill_Secondary`
  (params (Key :type "Key Structure" :default "AnyKey"))
  (:`Pressed`
    (goto _label_2 :!via `Press`))
  (:`Released`
    (goto _label_2 :!via `Release`)))

(event `self.ReceiveDestroyed`
  (bind _asbp_test_2dgame_state (cast `/Game/Blueprints/GameData/BP_Test2DGameState` (`GameplayStatics.GetGameState`)))
  (`KismetArrayLibrary.Array_RemoveItem` (`/Game/Blueprints/GameData/BP_Test2DGameState.Controllers` _asbp_test_2dgame_state) self))

(event `InputAction|Skill_Util_0`
  (params (Key :type "Key Structure" :default "AnyKey"))
  (:`Pressed`
    (goto _label_3 :!via `Press`))
  (:`Released`
    (goto _label_3 :!via `Release`)))

(event `InputAction|Skill_Util_1`
  (params (Key :type "Key Structure" :default "AnyKey"))
  (:`Pressed`
    (goto _label_4 :!via `Press`))
  (:`Released`
    (goto _label_4 :!via `Release`)))

(event `InputAction|Skill_Util_2`
  (params (Key :type "Key Structure" :default "AnyKey"))
  (:`Pressed`
    (goto _label_5 :!via `Press`))
  (:`Released`
    (goto _label_5 :!via `Release`)))

(event `InputAction|Skill_Dodge`
  (params (Key :type "Key Structure" :default "AnyKey"))
  (:`Pressed`
    (goto _label_6 :!via `Press`))
  (:`Released`
    (goto _label_6 :!via `Release`)))

(event `InputAction|Skill_Buff_0`
  (params (Key :type "Key Structure" :default "AnyKey"))
  (:`Pressed`
    (goto _label_7 :!via `Press`))
  (:`Released`
    (goto _label_7 :!via `Release`)))

(event `InputAction|Skill_Buff_1`
  (params (Key :type "Key Structure" :default "AnyKey"))
  (:`Pressed`
    (goto _label_8 :!via `Press`))
  (:`Released`
    (goto _label_8 :!via `Release`)))

(event `InputAction|Skill_Buff_2`
  (params (Key :type "Key Structure" :default "AnyKey"))
  (:`Pressed`
    (goto _label_9 :!via `Press`))
  (:`Released`
    (goto _label_9 :!via `Release`)))

(fn `Init`
  (bind _returnvalue (`self.K2_GetPawn`))
  (if (`KismetMathLibrary.ClassIsChildOf` (`GameplayStatics.GetObjectClass` _returnvalue) "/Game/Blueprints/Character/Player/BP_Player_Character.BP_Player_Character_C")
    (bind _asbp_player_character (cast `/Game/Blueprints/Character/Player/BP_Player_Character` _returnvalue))
    (bind _output_get (set `self.Base2DCharacter` _asbp_player_character))
    (bind _asbp_2dhu_d (cast `/Game/Blueprints/HuD/BP_2DHuD` (`self.GetHUD`)))
    (`/Game/Blueprints/HuD/BP_2DHuD.Init` _asbp_2dhu_d self _output_get)))

(fn `UserConstructionScript`)