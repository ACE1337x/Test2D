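; Player character for a 2D side-view game, driving the mouse-follow camera and aim direction and pulling its name from the game state.
; Each tick, UpdateMouse sizes the detached orthographic camera from viewport and zoom, deprojects the cursor and sets LookDir.
; The camera eases toward half the clamped player-to-cursor offset, floored to whole units.
; ToggleUpdateCamera switches cursor-following against a visible mouse cursor; name lookup retries while empty.
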(event `self.ReceiveBeginPlay`
  (`parent.ReceiveBeginPlay`)
  (`self.InitHudAndController`)
  (`self.Update Mouse` 0.0)
  (`self.SetupName`))

(event `self.ReceiveTick`
  (params (DeltaSeconds :type "Float (single-precision)"))
  (`parent.ReceiveTick` DeltaSeconds)
  (`|ExecutionSequence`
    (:`then_0`
      (`self.Update Mouse` DeltaSeconds))
    (:`then_1`
      (if (`KismetStringLibrary.EqualEqual_StrStr` (`self.Name`))
        (`self.SetupName`)))))

(event `Update Mouse`
  (params (Dt :type "Float (double-precision)"))
  (`self.UpdateMouse` Dt))

(event `self.SetupName`
  (bind _asbp_test_2dgame_state (cast `/Game/Blueprints/GameData/BP_Test2DGameState` (`GameplayStatics.GetGameState`)))
  (bind _returnvalue (`KismetArrayLibrary.Array_Find` (`/Game/Blueprints/GameData/BP_Test2DGameState.Controllers` _asbp_test_2dgame_state) (`self.GetController`)))
  (if (>= _returnvalue 0)
    (set `self.Name` (`KismetArrayLibrary.Array_Get` (`/Game/Blueprints/GameData/BP_Test2DGameState.Names` _asbp_test_2dgame_state) _returnvalue))
    (`parent.SetupName`)
    (else
      (`parent.SetupName`))))

(event `ToggleUpdateCamera`
  (params (Update :type Boolean))
  (set `self.UpdateCameraPos` Update)
  (set `PlayerController.bShowMouseCursor` (not Update) (`GameplayStatics.GetPlayerController` 0)))

(fn `UpdateMouse`
  (params (DeltaTime :type "Float (double-precision)"))
  (bind _returnvalue (`self.K2_GetActorLocation`))
  (bind _camera (`self.Camera`))
  (bind _maxcrosshairdistancefromplayer (`self.MaxCrosshairDistanceFromPlayer`))
  (bind _returnvalue_2 (/ (`self.ZoomFactor`) (`self.PixelsPerUU`)))
  (bind _returnvalue_3 (`KismetMathLibrary.MakeVector` (.x (- (select `bool` (`self.UpdateCameraPos`) :`false` (`self.K2_GetActorLocation`) :`true` (`self.MouseLocation`)) _returnvalue)) 0.0 (.z (- (select `bool` (`self.UpdateCameraPos`) :`false` (`self.K2_GetActorLocation`) :`true` (`self.MouseLocation`)) _returnvalue))))
  (bind _asplayer_controller (cast `PlayerController` (`self.GetController`)))
  (`|ExecutionSequence`
    (:`then_0`
      (bind (_sizex _sizey) (`PlayerController.GetViewportSize` _asplayer_controller))
      (bind _returnvalue_4 (`KismetMathLibrary.Conv_IntToDouble` _sizex))
      (`CameraComponent.SetOrthoWidth` _camera (/ _returnvalue_4 _returnvalue_2))
      (`CameraComponent.SetAspectRatio` _camera (/ _returnvalue_4 (`KismetMathLibrary.Conv_IntToDouble` _sizey)))
      (set `self.MaxCrosshairDistanceFromPlayer` (/ _returnvalue_4 (* _returnvalue_2 (`self.DistScalar`)))))
    (:`then_1`
      (bind (_worldlocation _worlddirection) (`PlayerController.DeprojectMousePositionToWorld` _asplayer_controller))
      (set `self.MouseLocation` (+ _worldlocation (* _worlddirection (`self.CameraDistance`))))
      (`SceneComponent.K2_SetWorldLocation` (`self.Camera`) (`KismetMathLibrary.MakeVector` (`KismetMathLibrary.Conv_IntToDouble` (`KismetMathLibrary.FFloor` (.x (`KismetMathLibrary.VInterpTo` (`SceneComponent.K2_GetComponentLocation` (`self.Camera`)) (+ (`KismetMathLibrary.MakeVector` (.x _returnvalue) 0.0 (.z _returnvalue)) (* (select `bool` (> (`KismetMathLibrary.VSize` _returnvalue_3) _maxcrosshairdistancefromplayer) :`false` _returnvalue_3 :`true` (* (`KismetMathLibrary.Normal` _returnvalue_3) _maxcrosshairdistancefromplayer)) 0.5)) DeltaTime 5.0)))) (`self.CameraDistance`) (`KismetMathLibrary.Conv_IntToDouble` (`KismetMathLibrary.FFloor` (.z (`KismetMathLibrary.VInterpTo` (`SceneComponent.K2_GetComponentLocation` (`self.Camera`)) (+ (`KismetMathLibrary.MakeVector` (.x _returnvalue) 0.0 (.z _returnvalue)) (* (select `bool` (> (`KismetMathLibrary.VSize` _returnvalue_3) _maxcrosshairdistancefromplayer) :`false` _returnvalue_3 :`true` (* (`KismetMathLibrary.Normal` _returnvalue_3) _maxcrosshairdistancefromplayer)) 0.5)) DeltaTime 5.0))))) false false)
      (set `self.lookDir` (`KismetMathLibrary.Normal` (- (`KismetMathLibrary.MakeVector` (.x (`self.MouseLocation`)) 0.0 (.z (`self.MouseLocation`))) (`KismetMathLibrary.MakeVector` (.x (`self.K2_GetActorLocation`)) 0.0 (.z (`self.K2_GetActorLocation`)))))))))

(fn `UserConstructionScript`
  (`parent.UserConstructionScript`)
  (`SceneComponent.DetachFromParent` (`self.Camera`) true true))