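; Base 2D character Blueprint that shows a name label and HP bar through widget components.
; On BeginPlay it runs the parent logic, fills the outlined name text and hands its AttributeComponent to the HP bar widget.
; The construction script drops SceneComponent to the capsule's bottom using the negative half-height.
; InitHudAndController calls Init on BP_PlayerController and is not invoked within this graph.
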(event `self.ReceiveBeginPlay`
  (`parent.ReceiveBeginPlay`)
  (`self.SetupName`)
  (`self.SetupHPBar`))

(fn `InitHudAndController`
  (bind _asbp_player_controller (cast `/Game/Blueprints/Character/Player/BP_PlayerController` (`self.GetController`)))
  (`/Game/Blueprints/Character/Player/BP_PlayerController.Init` _asbp_player_controller))

(fn `SetupHPBar`
  (bind _asbp_hp_bars (cast `/Game/Blueprints/HuD/HPBar/BP_HpBars` (`WidgetComponent.GetUserWidgetObject` (`self.HpBar_Widget`))))
  (set `/Game/Blueprints/HuD/HPBar/BP_HpBars.AttributeComponent` (`self.AttributeComponent`) _asbp_hp_bars)
  (`/Game/Blueprints/HuD/BP_OutlineFont.SetSize` (`/Game/Blueprints/HuD/HPBar/BP_HpBars.OutlineFont` _asbp_hp_bars) 6 1))

(fn `SetupName`
  (bind _asbp_outline_font (cast `/Game/Blueprints/HuD/BP_OutlineFont` (`WidgetComponent.GetUserWidgetObject` (`self.Name_Widget`))))
  (set `/Game/Blueprints/HuD/BP_OutlineFont.Text` (`KismetTextLibrary.Conv_StringToText` (`self.Name`)) _asbp_outline_font)
  (`/Game/Blueprints/HuD/BP_OutlineFont.SetSize` _asbp_outline_font 12 1))

(fn `SetupSceneCompLoc`
  (`SceneComponent.K2_SetRelativeLocation` (`self.SceneComponent`) (`KismetMathLibrary.MakeVector` 0.0 0.0 (* (`CapsuleComponent.CapsuleHalfHeight` (`self.CapsuleComponent`)) -1.0)) false true))

(fn `UserConstructionScript`
  (`self.SetupSceneCompLoc`))